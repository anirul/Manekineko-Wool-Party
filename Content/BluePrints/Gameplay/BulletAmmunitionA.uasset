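; BulletAmmunitionA is an ammunition pickup with a randomly colored sphere.
; On BeginPlay it picks a random bullet color enum entry and applies the matching yellow, blue or red material.
; When an actor of class 0_Base overlaps it, it tells its Spawner to begin spawning and then destroys itself.
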(event EventBeginPlay
  (CallFunction|InitBulletColor))

(event Collision|EventActorBeginOverlap
  (params (OtherActor :type Actor%20Object%20Reference))
  (Utilities|Casting|CastTo0_Base OtherActor)
  (Default|BeginSpawning (Variables|Default|GetSpawner))
  (Actor|DestroyActor))

(event EventTick
  (params (DeltaSeconds :type Float%20%28single-precision%29)))

(fn ConstructionScript)

(fn InitBulletColor
  (bind _sphere (Variables|Default|GetSphere))
  (bind _output_get (Variables|Default|SetColor (Utilities|Enum|ByteToEnumBulletColor (Math|Conversions|ToByte(Integer) (Math|Random|RandomInteger (|GetNumEnumEntries))))))
  (switch Utilities|FlowControl|Switch|SwitchonBulletColor _output_get
    (:NewEnumerator0
      (Rendering|Material|SetMaterial _sphere 0 "/Game/Materials/Yellow.Yellow"))
    (:NewEnumerator1
      (Rendering|Material|SetMaterial _sphere 0 "/Game/Materials/Blue.Blue"))
    (:NewEnumerator2
      (Rendering|Material|SetMaterial _sphere 0 "/Game/Materials/Red.Red"))))