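; Pickup spawner actor that places a BulletAmmunitionA actor 200 units above itself at BeginPlay.
; Each spawned ammunition receives a Spawner reference back to this actor.
; BeginSpawning, not called within this file, starts a Period-long countdown that Tick decrements, spawning a single replacement when it runs out.
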(event EventBeginPlay
  (CallFunction|SpawnNewBullet))

(event Collision|EventActorBeginOverlap
  (params (OtherActor :type Actor%20Object%20Reference)))

(event EventTick
  (params (DeltaSeconds :type Float%20%28single-precision%29))
  (CallFunction|CheckifNewSpawn DeltaSeconds))

(fn ConstructionScript)

(fn SpawnNewBullet
  (bind _returnvalue (Transformation|GetActorTransform))
  (bind (_location _rotation _scale) (Math|Transform|BreakTransform _returnvalue))
  (bind _returnvalue_2 (Game|SpawnActorfromClass "/Game/BluePrints/Gameplay/BulletAmmunitionA.BulletAmmunitionA_C" (Math|Transform|MakeTransform (+ _location "0, 0,200.000000") _rotation _scale) "Undefined" 0 0))
  (Variables|/Game/BluePrints/Gameplay/BulletAmmunitionA.BulletAmmunitionA_C|SetSpawner _returnvalue_2 self))

(fn CheckifNewSpawn
  (params (deltaSeconds :type Float%20%28single-precision%29))
  (if (Variables|Default|Getspawning)
    (bind _output_get (Variables|Default|Settimer (- (Variables|Default|Gettimer) deltaSeconds)))
    (if (< _output_get 0.0)
      (CallFunction|SpawnNewBullet)
      (Variables|Default|Setspawning false))))

(fn BeginSpawning
  (Variables|Default|Settimer (Variables|Default|Getperiod))
  (Variables|Default|Setspawning true))