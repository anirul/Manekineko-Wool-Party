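; Gameplay game mode that runs a timed match and handles player spawning and departure.
; On the authority, a timer set from the GameInfoInstance map time opens ScoreMap when it expires.
; RespawnPlayer destroys the controller's current pawn, then spawns and possesses the given character class at a random PlayerStart.
; It also records swapped-in player controllers and asks the game instance to destroy the session on logout.
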(event Custom|RespawnPlayer
  (params (Controller :type Player%20Controller%20Object%20Reference) (PlayerCharacter :type Character%20Class%20Reference))
  (bind _returnvalue (Pawn|GetControlledPawn Controller))
  ;[1 1 1] Spawn the player with their selected character from the controller
  (bind _outactors (Actor|GetAllActorsOfClass "/Script/Engine.PlayerStart"))
  (Variables|GameInfo|SetSpawnPoints _outactors)
  (Utilities|IsValid _returnvalue
    (:Is%20Valid
      (Actor|DestroyActor _returnvalue))
    (:Is%20Not%20Valid
      _))
  (bind _returnvalue_2 (Game|SpawnActorfromClass PlayerCharacter (Transformation|GetActorTransform (Utilities|Array|Get(acopy) (Variables|GameInfo|GetSpawnPoints) (Math|Random|RandomIntegerinRange 0 (- (Utilities|Array|Length (Variables|GameInfo|GetSpawnPoints)) 1)))) "Undefined" 0 0))
  (Pawn|Possess Controller _returnvalue_2)
  (Input|SetInputModeGameOnly (Game|GetPlayerController 0)))

(event Custom|EndMapTimer
  ;[1 1 1] Reset level when time is up
  (Game|OpenLevel(byName) "ScoreMap"))

(event EventOnSwapPlayerControllers
  (params (OldPC :type Player%20Controller%20Object%20Reference) (NewPC :type Player%20Controller%20Object%20Reference))
  ;[1 1 1] Keep track of player controller
  (Utilities|Array|Add (Variables|GameInfo|GetAllPlayerControllers) NewPC))

(event EventOnLogout
  (params (ExitingController :type Controller%20Object%20Reference))
  ;[1 1 1] On logout destroy controller in game instance
  (bind _asgame_play_pc (Utilities|Casting|CastToGamePlayPC ExitingController))
  (bind _asgame_info_instance (Utilities|Casting|CastToGameInfoInstance (Game|GetGameInstance)))
  (Default|DestroySessionCaller _asgame_info_instance _asgame_play_pc))

(event EventBeginPlay
  ;[1 1 1] Reset level when time is up
  (Networking|SwitchHasAuthority
    (:Authority
      (bind _asgame_info_instance (Utilities|Casting|CastToGameInfoInstance (Game|GetGameInstance)))
      (Utilities|Time|SetTimerbyEvent (delegate Custom|EndMapTimer) (Variables|/Game/BluePrints/AllLevels/GameINfoInstance.GameInfoInstance_C|GetMapTime _asgame_info_instance)))))

(fn ConstructionScript)