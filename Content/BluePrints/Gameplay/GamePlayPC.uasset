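; Gameplay player controller that spawns the player's chosen character, owns the HUD and tracks a capped queue of colored ammunition.
; On local BeginPlay it loads saved player settings and passes them to the server, which asks GamePlayGM to respawn the player, then sets up the HUD.
; Ammunition is appended up to a maximum and removed from the front when shot, updating the HUD on each change.
; Escape quits the game.
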(event Custom|PassCharacterInfoToServer
  (params (PlayerSetting :type Player%20Info%20Structure))
  ;[1 1 1] Passes character info - respawn player with selected character setup chat window
  (Variables|Default|SetPlayerSettings PlayerSetting)
  (bind _asgame_play_gm (Utilities|Casting|CastToGamePlayGM (Game|GetGameMode)))
  (Default|RespawnPlayer _asgame_play_gm self (.MyPlayerCharacter (Utilities|Struct|BreakPlayerInfo (Variables|Default|GetPlayerSettings))))
  (CallFunction|SetupGameplayWindow))

(event Custom|SetupGameplayWindow
  ;[1 1 1] Create Gameplay HUD
  (bind _returnvalue (UserInterface|CreateWidget "/Game/UI/Gameplay/GameplayHUD.GameplayHUD_C"))
  (bind _output_get (Variables|Default|SetGameplayWB _returnvalue))
  (UserInterface|Viewport|AddtoViewport _output_get 0))

(event Custom|AddAmmunition
  (params (NewColor :type BulletColor%20Enum))
  (CallFunction|AddNewAmmunition NewColor))

(event Custom|Replicate%20Ammunition
  (params (Ammunitions :type Array%20of%20BulletColor%20Enums))
  (bind _output_get (Variables|Default|SetAmmunitions Ammunitions))
  (Default|UpdateAmmunition (Variables|Default|GetGameplayWB) _output_get))

(event EventBeginPlay
  ;[1 1 1] Load Player Info and pass it to server Controller
  (if (Pawn|IsLocalController)
    (Viewport|RemoveAllWidgets)
    (CallFunction|LoadGame)
    (CallFunction|PassCharacterInfotoServer (Variables|Default|GetPlayerSettings))))

(event Input|KeyboardEvents|Escape
  (params (Key :type Key%20Structure :default "AnyKey"))
  ;[1 1 1] Quit on escape
  (:Pressed
    (Game|QuitGame 0 "Quit")))

(fn ConstructionScript)

(fn LoadGame
  (bind _returnvalue (SaveGame|LoadGamefromSlot (Variables|Default|GetPlayerSettingsSave)))
  (bind _asplayer_save_game (Utilities|Casting|CastToPlayerSaveGame _returnvalue))
  (Variables|Default|SetPlayerSettings (Variables|/Game/BluePrints/AllLevels/PlayerSaveGame.PlayerSaveGame_C|GetS_PlayerInfo _asplayer_save_game)))

(fn AddNewAmmunition
  (params (NewColor :type BulletColor%20Enum))
  (bind _ammunitions (Variables|Default|GetAmmunitions))
  (if (< (Utilities|Array|Length _ammunitions) (Variables|Default|GetMaxAmmunition))
    (Utilities|Array|Add _ammunitions NewColor)
    (CallFunction|ReplicateAmmunition (Variables|Default|GetAmmunitions))))

(fn ShootAmmunition
  (bind _ammunitions (Variables|Default|GetAmmunitions))
  (if (!= (Utilities|Array|Length _ammunitions) 0)
    (Utilities|Array|RemoveIndex _ammunitions)
    (Default|UpdateAmmunition (Variables|Default|GetGameplayWB) _ammunitions)))