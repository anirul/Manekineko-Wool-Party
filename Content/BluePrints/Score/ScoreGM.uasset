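; ScoreGM is the Blueprint behind the score screen, listing player results and offering a way back to the main menu.
; On BeginPlay it creates the ScoreUI widget and fills its PlayerList with one PlayerScore widget per PlayerInfoScore entry from GameInfoInstance.
; It then shows the widget with the mouse cursor and UI-only input.
; An ExitToMainMenu event opens MainMenuMap.
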(event Custom|ExitToMainMenu
  ;[1 1 1] Exit to main menu
  (Game|OpenLevel(byName) "MainMenuMap"))

(event EventBeginPlay
  (bind _returnvalue (Game|GetPlayerController 0))
  ;[1 1 1] Create the score screen and add it to viewport
  (Utilities|IsValid (Variables|Default|GetScoreWB)
    (:Is%20Valid
      _)
    (:Is%20Not%20Valid
      (bind _returnvalue_2 (UserInterface|CreateWidget "/Game/UI/Score/ScoreUI.ScoreUI_C"))
      (Variables|Default|SetScoreWB _returnvalue_2)))
  (bind _asgame_info_instance (Utilities|Casting|CastToGameInfoInstance (Game|GetGameInstance)))
  (Widget|Panel|ClearChildren (Variables|/Game/UI/Score/ScoreUI.ScoreUI_C|GetPlayerList (Variables|Default|GetScoreWB)))
  (for _array_element (Variables|/Game/BluePrints/AllLevels/GameINfoInstance.GameInfoInstance_C|GetPlayerInfoScore _asgame_info_instance)
    (bind _returnvalue_3 (UserInterface|CreateWidget "/Game/UI/Score/PlayerScore.PlayerScore_C" 0 _array_element))
    (Widget|Panel|AddChild (Variables|/Game/UI/Score/ScoreUI.ScoreUI_C|GetPlayerList (Variables|Default|GetScoreWB)) _returnvalue_3))
  (UserInterface|Viewport|AddtoViewport (Variables|Default|GetScoreWB) 0)
  (Variables|/Script/Engine.PlayerController|SetbShowMouseCursor _returnvalue true)
  (Input|SetInputModeUIOnly _returnvalue (Variables|Default|GetScoreWB) "DoNotLock"))

(fn ConstructionScript)